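; Enemy AI character that chases the player on sight, performs melee attacks and takes damage.
; Pawn sensing sets a seen flag that is never effectively cleared and starts AIMoveTo; arrival triggers a delayed attack.
; The attack calls a montage and applies damage through a debug-drawn line trace between two components.
; Incoming damage reduces health; a hit at zero or below ragdolls the mesh and destroys the capsule.
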(event `self.ReceiveTick`
  (params (DeltaSeconds :type "Float (single-precision)"))
  ;[1 1 1] Attack + Follow
  (if (not (`self.Is_Seeing_Player`))
    (`MovementComponent.StopMovementImmediately` (`self.CharacterMovement`))))

(event `self.PawnSensing.OnSeePawn`
  (params (Pawn :type "Pawn Object Reference"))
  ;[1 1 1] Attack + Follow
  (set `self.Is_Seeing_Player` true)
  (`self.FollowPlayer`))

(event `FollowPlayer`
  ;[1 1 1] Attack + Follow
  (set `self.can_Attack?` true)
  (if (`self.Is_Seeing_Player`)
    (`|AIMoveTo` self (0.0 0.0 0.0) (`GameplayStatics.GetPlayerCharacter` 0) 17.0
      (:`OnSuccess`
        (if (`self.can_Attack?`)
          (set `self.can_Attack?` false)
          (`KismetSystemLibrary.Delay` 1.0)
          (`self.EnemyAttack`))))
    (else
      (set `self.Is_Seeing_Player` false))))

(event `EnemyAttack`
  ;[1 1 1] Attack + Follow
  (`self.PlayAnimMontage` null)
  (bind _outhit (`KismetSystemLibrary.LineTraceSingle` :`Start` (`SceneComponent.GetSocketLocation` (`self.StartAttack`) "None") :`End` (`SceneComponent.GetSocketLocation` (`self.EndAttack`) "None") :`TraceChannel` "TraceTypeQuery1" :`DrawDebugType` "ForDuration"))
  (`GameplayStatics.ApplyDamage` (`.HitActor` (`GameplayStatics.BreakHitResult` _outhit)) 2.0))

(event `self.ReceiveAnyDamage`
  (params (Damage :type "Float (single-precision)") (DamageType :type "DamageType Object Reference") (InstigatedBy :type "Controller Object Reference") (DamageCauser :type "Actor Object Reference"))
  ;[1 1 1] taking Damagae
  (if (> (`self.Health`) 0.0)
    (set `self.Health` (- (`self.Health`) Damage))
    (`KismetSystemLibrary.PrintString` "Enemy Hit")
    (else
      (`PrimitiveComponent.SetSimulatePhysics` (`self.Mesh`) true)
      (`ActorComponent.K2_DestroyComponent` (`self.CapsuleComponent`))
      (`KismetSystemLibrary.Delay` 2.0))))

(fn `UserConstructionScript`)