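; Melee enemy character that chases the player on sight, punches on reaching them, takes damage and ragdolls when its health runs out.
; Pawn sensing starts an AI MoveTo, whose success triggers a timer-reset punch animation and briefly enables a hit box's overlap events.
; Box overlaps with the player apply damage, sound, particles, camera shake and an actor attachment to a fist socket.
; Tazer projectile hits disable movement and play a stun animation for several seconds.
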(event `self.ReceiveTick`
  (params (DeltaSeconds :type "Float (single-precision)"))
  ;[1 1 1] Attack + Follow
  (if (not (`self.Is_Seeing_Player`))
    (`MovementComponent.StopMovementImmediately` (`self.CharacterMovement`))))

(event `self.PawnSensing.OnSeePawn`
  (params (Pawn :type "Pawn Object Reference"))
  ;[1 1 1] Attack + Follow
  (set `self.Is_Seeing_Player` true)
  (`self.FollowPlayer`))

(event `FollowPlayer`
  ;[1 1 1] Attack + Follow
  (set `self.can_Attack?` true)
  (if (`self.Is_Seeing_Player`)
    (`|AIMoveTo` self (0.0 0.0 0.0) (`GameplayStatics.GetPlayerCharacter` 0) 17.0
      (:`OnSuccess`
        (if (`self.can_Attack?`)
          (set `self.can_Attack?` false)
          (`KismetSystemLibrary.Delay` 0.5)
          (`self.EnemyAttack`)
          (`/Engine/EditorBlueprintResources/StandardMacros.DoOnce` false :!label _label
            (:`Completed`
              (`|ExecutionSequence`
                (:`then_0`
                  (`MovementComponent.StopMovementImmediately` (`self.CharacterMovement`))
                  (`SkeletalMeshComponent.PlayAnimation` (`self.Mesh`) "/Game/Characters/Mannequins/Animations/Manny/Arm_punch-stretch.Arm_punch-stretch" false)
                  (`KismetSystemLibrary.Delay` 0.5)
                  (`CharacterMovementComponent.SetMovementMode` (`self.CharacterMovement`) "MOVE_Walking" 0)
                  (`SkeletalMeshComponent.SetAnimationMode` (`self.Mesh`) "AnimationBlueprint"))
                (:`then_1`
                  (`KismetSystemLibrary.K2_SetTimerDelegate` (delegate `Reset_Attack`) 0.5))))))))
    (else
      (set `self.Is_Seeing_Player` false))))

(event `Reset_Attack`
  ;[1 1 1] Attack + Follow
  (goto _label :!via `Reset`))

(event `EnemyAttack`
  (bind _box (`self.Box`))
  ;[1 1 1] Attack + Follow
  (set `PrimitiveComponent.bGenerateOverlapEvents` true _box)
  (`KismetSystemLibrary.Delay` 0.5)
  (set `PrimitiveComponent.bGenerateOverlapEvents` false _box))

(event `self.ReceiveBeginPlay`
  ;[1 1 1] Attack + Follow
  (set `PrimitiveComponent.bGenerateOverlapEvents` false (`self.Box`))
  (set `self.Stunned` true))

(event `self.ReceiveAnyDamage`
  (params (Damage :type "Float (single-precision)") (DamageType :type "DamageType Object Reference") (InstigatedBy :type "Controller Object Reference") (DamageCauser :type "Actor Object Reference"))
  ;[1 1 1] taking Damagae
  (if (> (`self.Health`) 0.0)
    (set `self.Health` (- (`self.Health`) Damage))
    (`KismetSystemLibrary.PrintString` "Enemy Hit")
    (else
      (`PrimitiveComponent.SetSimulatePhysics` (`self.Mesh`) true)
      (`ActorComponent.K2_DestroyComponent` (`self.CapsuleComponent`))
      (`PrimitiveComponent.SetCollisionResponseToChannel` (`self.Mesh`) "ECC_WorldDynamic" "ECR_Ignore"))))

(event `self.Box.OnComponentBeginOverlap`
  (params (OverlappedComponent :type "PrimitiveComponent Object Reference") (OtherActor :type "Actor Object Reference") (OtherComp :type "PrimitiveComponent Object Reference") (OtherBodyIndex :type Integer) (bFromSweep :type Boolean) (SweepResult :type "HitResult Structure (by ref)"))
  ;[1 1 1] Punch
  (if (== (`GameplayStatics.GetObjectClass` OtherActor) "/Game/TopDown/Blueprints/BP_TopDownCharacter.BP_TopDownCharacter_C")
    (`GameplayStatics.ApplyDamage` OtherActor 1.0)
    (`GameplayStatics.PlaySound2D` "/Game/Sujais_file/Sujais_Sound_Audios/Chaz-_Sounds/punch.punch" 1.0 1.0 0.0 null null)
    (`ActorComponent.Activate` (`self.ParticleSystem`) true)
    (bind _asbp_top_down_character (cast `/Game/TopDown/Blueprints/BP_TopDownCharacter` (`GameplayStatics.GetPlayerPawn` 0)))
    (`self.K2_AttachToActor` _asbp_top_down_character "Fist" "KeepWorld" "KeepRelative" "KeepWorld")
    ;;[0 0.1964 1] need diffrent values/intervals
    (`GameplayStatics.PlayWorldCameraShake` "/Game/TopDown/Blueprints/BP_Punch_Shake.BP_Punch_Shake_C" (`self.K2_GetActorLocation`) 0.0 3000.0)
    (`KismetSystemLibrary.PrintString` "Player hit")))

(event `self.ReceiveHit`
  (params (MyComp :type "PrimitiveComponent Object Reference") (Other :type "Actor Object Reference") (OtherComp :type "PrimitiveComponent Object Reference") (bSelfMoved :type Boolean) (HitLocation :type "Vector Structure") (HitNormal :type "Vector Structure") (NormalImpulse :type "Vector Structure") (Hit :type "HitResult Structure (by ref)"))
  ;[1 1 1] Tazer Stun
  (cast `/Game/Weapons+Items/BP_tazer_projectile` Other)
  (`CharacterMovementComponent.DisableMovement` (`self.CharacterMovement`))
  (`GameplayStatics.PlaySound2D` "/Game/Sujais_file/Sujais_Sound_Audios/Chaz-_Sounds/electrictysparks.electrictysparks" 1.0 1.0 0.0 null null)
  (`SkeletalMeshComponent.PlayAnimation` (`self.Mesh`) "/Game/Characters/Mannequins/Animations/Manny/SK_Mannequin_Sequence_Stunned.SK_Mannequin_Sequence_Stunned" (`self.Stunned`))
  (`KismetSystemLibrary.Delay` 5.0)
  (`SkeletalMeshComponent.PlayAnimation` (`self.Mesh`) "/Game/Characters/Mannequins/Animations/Quinn/MF_Run_Fwd.MF_Run_Fwd" true)
  (`CharacterMovementComponent.SetMovementMode` (`self.CharacterMovement`) "MOVE_Walking" 0))

(event `self.ReceiveActorBeginOverlap`
  (params (OtherActor :type "Actor Object Reference"))
  ;[1 1 1] Tazer Stun
  (if (== (`GameplayStatics.GetObjectClass` OtherActor) "/Game/Weapons+Items/BP_tazer_projectile.BP_tazer_projectile_C")
    (set `self.Stunned` true)
    (`KismetSystemLibrary.Delay` 5.0)
    (set `self.Stunned` false)))

(fn `UserConstructionScript`)