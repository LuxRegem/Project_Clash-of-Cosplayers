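; Club pickup item that acts as a melee weapon against melee enemies.
; On BeginPlay its static mesh is set to ignore the player pawn when moving.
; Item activation opens a brief hit window by toggling overlap events on a capsule with a delay.
; A melee enemy overlapping the capsule is reported to the player pawn through an ItemHitThingMessage call, leaving the hit response to the pawn.
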(event `self.ReceiveBeginPlay`
  (`parent.ReceiveBeginPlay`)
  (`PrimitiveComponent.IgnoreActorWhenMoving` (`self.StaticMesh`) (`GameplayStatics.GetPlayerPawn` 0) true))

(event `/Game/Lukes_Content/Interaction/Interaction_Interface.ItemActivation`
  (bind _capsule (`self.Capsule`))
  (set `PrimitiveComponent.bGenerateOverlapEvents` true _capsule)
  (`KismetSystemLibrary.Delay` 0.5)
  (set `PrimitiveComponent.bGenerateOverlapEvents` false _capsule))

(event `self.Cylinder.OnComponentBeginOverlap`
  (params (OverlappedComponent :type "PrimitiveComponent Object Reference") (OtherActor :type "Actor Object Reference") (OtherComp :type "PrimitiveComponent Object Reference") (OtherBodyIndex :type Integer) (bFromSweep :type Boolean) (SweepResult :type "HitResult Structure (by ref)")))

(event `self.Capsule.OnComponentBeginOverlap`
  (params (OverlappedComponent :type "PrimitiveComponent Object Reference") (OtherActor :type "Actor Object Reference") (OtherComp :type "PrimitiveComponent Object Reference") (OtherBodyIndex :type Integer) (bFromSweep :type Boolean) (SweepResult :type "HitResult Structure (by ref)"))
  (if (== (`GameplayStatics.GetObjectClass` OtherActor) "/Game/Enemy_AI/BluePrints/Enemy_Character_melee.Enemy_Character_melee_C")
    (message `/Game/Lukes_Content/Interaction/Interaction_Interface.ItemHitThing` (`GameplayStatics.GetPlayerPawn` 0) OtherActor)))

(fn `UserConstructionScript`
  (`parent.UserConstructionScript`))